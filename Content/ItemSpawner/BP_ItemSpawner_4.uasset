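; BP_ItemSpawner_4 is an item spawner actor that places a random item at its own location and rotation.
; BeginPlay sets a two-second timer that calls SpawnItem by function name.
; SpawnItem picks a random class from ItemsToSpawn, spawns it with collision adjustment that always spawns, and stores it in CurrentItem.
; The AttemptToSpawn function is an empty stub.
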(event `self.ReceiveBeginPlay`
  (`KismetSystemLibrary.K2_SetTimer` null "SpawnItem" 2.0))

(fn `Attempt to Spawn`)

(fn `SpawnItem`
  (bind _returnvalue (`|SpawnActorFromClass` (`|GetArrayItem` (`self.ItemsToSpawn`) (`KismetMathLibrary.RandomIntegerInRange` 0 (- (`KismetArrayLibrary.Array_Length` (`self.ItemsToSpawn`)) 1))) (`KismetMathLibrary.MakeTransform` (`self.K2_GetActorLocation`) (`self.K2_GetActorRotation`)) "AdjustIfPossibleButAlwaysSpawn" "OverrideRootScale" null null))
  (set `self.CurrentItem` _returnvalue))

(fn `UserConstructionScript`)