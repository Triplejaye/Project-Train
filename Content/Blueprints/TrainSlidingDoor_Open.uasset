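; Sliding train door whose two panels open when the first-person character enters its collision volume and close when the character leaves.
; After a short delay, end overlap plays a single timeline forward and begin overlap reverses it.
; The timeline track lerps both static mesh panels along local Y between mirrored side offsets and the centered position.
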(event `self.CollisionComp.OnComponentEndOverlap`
  (params (OverlappedComponent :type "PrimitiveComponent Object Reference") (OtherActor :type "Actor Object Reference") (OtherComp :type "PrimitiveComponent Object Reference") (OtherBodyIndex :type Integer))
  (cast `/Game/FirstPersonBP/Blueprints/FirstPersonCharacter` OtherActor)
  (`KismetSystemLibrary.Delay` 0.2)
  (bind (_direction _newtrack_0) (`Timeline|Timeline_0` :!label _label)
    (:`Update`
      (`SceneComponent.K2_SetRelativeLocation` (`self.StaticMeshComponent1`) (`KismetMathLibrary.VLerp` (0.0 120.0 0.0) (0.0 0.0 0.0) _newtrack_0) false false)
      (`SceneComponent.K2_SetRelativeLocation` (`self.StaticMeshComponent0`) (`KismetMathLibrary.VLerp` (0.0 -120.0 0.0) (0.0 0.0 0.0) _newtrack_0) false false))))

(event `self.CollisionComp.OnComponentBeginOverlap`
  (params (OverlappedComponent :type "PrimitiveComponent Object Reference") (OtherActor :type "Actor Object Reference") (OtherComp :type "PrimitiveComponent Object Reference") (OtherBodyIndex :type Integer) (bFromSweep :type Boolean) (SweepResult :type "HitResult Structure (by ref)"))
  (cast `/Game/FirstPersonBP/Blueprints/FirstPersonCharacter` OtherActor)
  (`KismetSystemLibrary.Delay` 0.2)
  (goto _label :!via `Reverse`))

(fn `UserConstructionScript`)